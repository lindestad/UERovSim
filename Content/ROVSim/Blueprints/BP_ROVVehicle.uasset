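; BP_ROVVehicle is a remotely operated vehicle Blueprint that turns keyboard input into movement commands.
; W/S set forward input and Space/Left Ctrl set vertical input, with each key release zeroing its axis.
; Every key change calls UpdateControlCommand, which packs both values into an ROV control command for SetControlCommand.
; Lateral and angular components are always zero, and no Tick logic is used.
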(event Custom|UpdateControlCommand
  (Class|ROVVehicle|SetControlCommand (Utilities|Struct|MakeROVControlCommand (Math|Vector|MakeVector (Variables|Default|GetFowardInput) 0.0 (Variables|Default|GetVerticalInput)) (Math|Vector|MakeVector 0.0 0.0 0.0))))

(event EventBeginPlay)

(event Collision|EventActorBeginOverlap
  (params (OtherActor :type Actor%20Object%20Reference)))

(event EventTick
  (params (DeltaSeconds :type Float%20%28single-precision%29)))

(event Input|KeyboardEvents|W
  (params (Key :type Key%20Structure :default "None"))
  (:Pressed
    (Variables|Default|SetFowardInput 1.0)
    (CallFunction|UpdateControlCommand))
  (:Released
    (Variables|Default|SetFowardInput 0.0)
    (CallFunction|UpdateControlCommand)))

(event Input|KeyboardEvents|S
  (params (Key :type Key%20Structure :default "None"))
  (:Pressed
    (Variables|Default|SetFowardInput -1.0)
    (CallFunction|UpdateControlCommand))
  (:Released
    (Variables|Default|SetFowardInput 0.0)
    (CallFunction|UpdateControlCommand)))

(event Input|KeyboardEvents|SpaceBar
  (params (Key :type Key%20Structure :default "None"))
  (:Pressed
    (Variables|Default|SetVerticalInput 1.0)
    (CallFunction|UpdateControlCommand))
  (:Released
    (Variables|Default|SetVerticalInput 0.0)
    (CallFunction|UpdateControlCommand)))

(event Input|KeyboardEvents|LeftCtrl
  (params (Key :type Key%20Structure :default "None"))
  (:Pressed
    (Variables|Default|SetVerticalInput -1.0)
    (CallFunction|UpdateControlCommand))
  (:Released
    (Variables|Default|SetVerticalInput 0.0)
    (CallFunction|UpdateControlCommand)))

(fn ConstructionScript)